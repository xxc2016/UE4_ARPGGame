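; BP_BladeCharacter is a twin-blade melee character with health, shared by input and AI attacks, though a note marks the Blueprint attack as superseded by C++.
; Weapon sockets get boxes at BeginPlay, and montage notifies run a timer line-tracing between their previous and current positions.
; Hits on differently tagged blade characters deal damage and play directional reactions chosen by dot products.
; Tick updates the health bar and handles death with delayed destruction.
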(event `InputAction|Attack`
  (params (Key :type "Key Structure"))
  ;[1 1 1] 攻击//c++以实现，蓝图作废
  (:`Pressed`
    (bind (_charactermovement _returnvalue) (`self.CanAttack?` :!label _label))
    (if _returnvalue
      (set `self.IsAttacking` true)
      (`CharacterMovementComponent.SetMovementMode` _charactermovement "MOVE_None" 0)
      (`|PlayMontage` (`self.Mesh`) "/Game/Animations/TwinBladeAttack_A1.TwinBladeAttack_A1" 1.0 0.0 "Attack_Start"
        (:`OnBlendOut`
          (if (not (== (`self.GetCurrentMontage`) "/Game/Animations/TwinBladeAttack_A1.TwinBladeAttack_A1")) :!label _label_2
            (`CharacterMovementComponent.SetMovementMode` _charactermovement "MOVE_Walking" 0)
            (set `self.IsAttacking` false)))
        (:`OnInterrupted`
          (goto _label_2))
        (:`OnNotifyBegin`
          ;[1 1 1] 攻击线段碰撞
          (`self.GetTracePosition`)
          (bind _returnvalue_2 (`KismetSystemLibrary.K2_SetTimerDelegate` (delegate `自定义事件_0`) 0.01 true))
          (set `self.Timer_0` _returnvalue_2))
        (:`OnNotifyEnd`
          (`KismetSystemLibrary.K2_ClearAndInvalidateTimerHandle` (`self.Timer_0`)))))))

(event `AI Attack`
  ;[1 1 1] 攻击//c++以实现，蓝图作废
  (goto _label))

(event `self.ReceiveBeginPlay`
  ;[1 1 1] 给武器插槽添加碰撞体
  (`|ExecutionSequence`
    (:`then_1`
      (`self.AddCollision`))))

(event `自定义事件_0`
  ;[1 1 1] 攻击线段碰撞
  (for (_array_element _array_index) (`self.Trace Collision_0`)
    (bind _outhits (`KismetSystemLibrary.LineTraceMultiForObjects` (`|GetArrayItem` (`self.TracePosition_0`) _array_index) (`SceneComponent.K2_GetComponentLocation` _array_element) (`self.Object Types_0`)))
    (for _array_element_2 _outhits
      ;[1 1 1] 播放受击动画
      (bind _asbp_blade_character (cast `/Game/Blueprints/BP_BladeCharacter` (`.HitActor` (`GameplayStatics.BreakHitResult` _array_element_2))))
      (if (not (or (`self.ActorHasTag` _asbp_blade_character (`|GetArrayItem` (`self.Tags`))) (== (`self.GetCurrentMontage` _asbp_blade_character) "/Game/Animations/HIT_Montage.HIT_Montage")))
        (`self.TakeDamage` _asbp_blade_character (`self.Damage_0`))
        (bind _mesh (`Character.Mesh` _asbp_blade_character))
        (bind _returnvalue (- (`SceneComponent.K2_GetComponentLocation` (`self.Mesh`)) (`SceneComponent.K2_GetComponentLocation` _mesh)))
        (bind _returnvalue_2 (`KismetMathLibrary.Dot_VectorVector` _returnvalue (`SceneComponent.GetForwardVector` _mesh)))
        (if (>= _returnvalue_2 0.86)
          (bind _mesh_2 (`Character.Mesh` _asbp_blade_character))
          (`|PlayMontage` _mesh_2 "/Game/Animations/HIT_Montage.HIT_Montage" 1.0 0.0 "Back")
          (elif (<= _returnvalue_2 -0.86)
            (`|PlayMontage` _mesh_2 "/Game/Animations/HIT_Montage.HIT_Montage" 1.0 0.0 "Front")
            (elif (>= (`KismetMathLibrary.Dot_VectorVector` _returnvalue (`SceneComponent.GetRightVector` _mesh)) 0.0)
              (`|PlayMontage` _mesh_2 "/Game/Animations/HIT_Montage.HIT_Montage" 1.0 0.0 "Left")
              (else
                (`|PlayMontage` _mesh_2 "/Game/Animations/HIT_Montage.HIT_Montage" 1.0 0.0 "Right"))))))))
  (`self.GetTracePosition`))

(event `self.ReceiveTick`
  (params (DeltaSeconds :type "Float (single-precision)"))
  (bind _health_0 (`self.Health_0`))
  ;[1 1 1] 血量与UI同步
  (`|ExecutionSequence`
    (:`then_0`
      (bind _aswb_health_bar (cast `/Game/Blueprints/BP_WB/WB_HealthBar` (`WidgetComponent.GetUserWidgetObject` (`self.HealthBar`))))
      (set `/Game/Blueprints/BP_WB/WB_HealthBar.HealthRatio` (/ _health_0 100.0) _aswb_health_bar))
    (:`then_1`
      (if (<= _health_0 0.0)
        (`/Engine/EditorBlueprintResources/StandardMacros.DoOnce` false
          (:`Completed`
            (`|ExecutionSequence`
              (:`then_0`
                (set `self.IsDead?` true)
                (`MovementComponent.StopMovementImmediately` (`self.CharacterMovement`))
                (`PrimitiveComponent.SetCollisionEnabled` (`self.CapsuleComponent`) "NoCollision"))
              (:`then_1`
                (`ActorComponent.Deactivate` (`self.CharacterMovement`))
                (`KismetSystemLibrary.Delay` 5.0)
                (`self.K2_DestroyActor`)))))))))

(fn `AddCollision`
  (bind _weapon_twinblade (`self.Weapon_Twinblade`))
  (for _array_element (`SceneComponent.GetAllSocketNames` _weapon_twinblade)
    (if (not (== _array_element "polySurface2"))
      (bind _returnvalue (`AddComponent|NODE_AddBoxComponent-0` :`RelativeTransform` (`SceneComponent.GetSocketTransform` _weapon_twinblade _array_element "RTS_Component")))
      (`KismetArrayLibrary.Array_Add` (`self.Trace Collision_0`) _returnvalue)
      (`SceneComponent.K2_AttachToComponent` _returnvalue (`self.Weapon_Twinblade`) "None" "KeepRelative" "KeepRelative" "KeepRelative" true)
      (for _array_element_2 (`self.Trace Collision_0`)
        (`KismetArrayLibrary.Array_Add` (`self.TracePosition_0`) (`SceneComponent.K2_GetComponentLocation` _array_element_2))))))

(fn `CanAttack?`
  (returns (CharacterMovement :type "CharacterMovementComponent Object Reference") (ReturnValue :type Boolean))
  (bind _charactermovement (`self.CharacterMovement`))
  (return _charactermovement (and (`|EnumEquality` (`CharacterMovementComponent.MovementMode` _charactermovement) "MOVE_Walking") (and (== (`self.GetCurrentMontage`) null) (not (`self.IsDead?`))))))

(fn `GetTracePosition`
  (for (_array_element _array_index) (`self.Trace Collision_0`)
    (`KismetArrayLibrary.Array_Set` (`self.TracePosition_0`) _array_index (`SceneComponent.K2_GetComponentLocation` _array_element))))

(fn `TakeDamage`
  (params (Damage :type "Float (double-precision)"))
  (bind _output_get (set `self.Health_0` (- (`self.Health_0`) Damage)))
  (`KismetSystemLibrary.PrintString` (`KismetStringLibrary.Conv_DoubleToString` _output_get)))

(fn `UserConstructionScript`)