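; Enemy AI controller that sets up the blackboard and runs the BT_Task behavior tree on BeginPlay.
; It stores the first player's pawn as TargetActor and writes an integer ActorType to the BB_Task blackboard.
; GetActorType derives that integer by checking whether the owner of ActionsComp is exactly BP_BladeEnemy, separating blade enemies from all other types.
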(event `self.ReceiveBeginPlay`
  (bind _blackboardcomponent (`self.UseBlackboard` "/Game/Blueprints/BP_Enemy/BB_Task.BB_Task"))
  (`BlackboardComponent.SetValueAsObject` _blackboardcomponent (`self.TargetActor`) (`GameplayStatics.GetPlayerPawn` 0))
  (bind _type (`self.GetActorType`))
  (`BlackboardComponent.SetValueAsInt` _blackboardcomponent (`self.ActorType`) _type)
  (`self.RunBehaviorTree` "/Game/Blueprints/BP_Enemy/BT_Task.BT_Task"))

(fn `GetActorType`
  (returns (Type :type Integer))
  (locals (NewLocalVar_0 :type Integer :default 1))
  (if (== (`GameplayStatics.GetObjectClass` (`ActorComponent.GetOwner` (`self.ActionsComp`))) "/Game/Blueprints/BP_Enemy/BP_BladeEnemy.BP_BladeEnemy_C")
    (set `local.NewLocalVar_0` 0)
    (else
      (set `local.NewLocalVar_0` 1)))
  (return (`local.NewLocalVar_0`)))

(fn `UserConstructionScript`)