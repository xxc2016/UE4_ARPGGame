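; Blade-wielding enemy Blueprint that feeds combat state to its AI controller's Blackboard.
; BeginPlay calls AddCollision, and Tick runs the parent logic before updating the Blackboard.
; CanAttack is true while the player pawn is within close 2D range of the enemy's mesh, and false when no pawn exists.
; IsDead is copied to the Blackboard only while a player pawn exists.
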(event `self.ReceiveBeginPlay`
  ;[1 1 1] 注释
  (`self.AddCollision`))

(event `self.ReceiveTick`
  (params (DeltaSeconds :type "Float (single-precision)"))
  (bind _returnvalue (`GameplayStatics.GetPlayerPawn` 0))
  (bind _returnvalue_2 (`AIBlueprintHelperLibrary.GetBlackboard` (`AIBlueprintHelperLibrary.GetAIController` self)))
  ;[1 1 1] 注释
  (`parent.ReceiveTick` 0.0)
  (if (!= _returnvalue null)
    (`BlackboardComponent.SetValueAsBool` _returnvalue_2 (`self.CanAttack?_0`) (<= (`KismetMathLibrary.Vector_Distance2D` (`SceneComponent.K2_GetComponentLocation` (`self.Mesh`)) (`self.K2_GetActorLocation` _returnvalue)) 100.0))
    (`BlackboardComponent.SetValueAsBool` _returnvalue_2 (`self.IsDead?_0`) (`self.IsDead?`))
    (else
      (`BlackboardComponent.SetValueAsBool` _returnvalue_2 (`self.CanAttack?_0`) false))))

(fn `UserConstructionScript`)