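; Ranged enemy character that feeds its AI blackboard and throws fireballs at the player.
; Tick writes death state and whether the player is within 2D attack range.
; AIAttack, commented as superseded by C++, halts movement during a montage whose notify launches a fireball from the Torch socket.
; Fireball hits damage BP_BladeCharacter unless tagged or already reacting, choosing a directional hit section via dot products against the enemy's position.
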(event `self.ReceiveTick`
  (params (DeltaSeconds :type "Float (single-precision)"))
  (bind _returnvalue (`GameplayStatics.GetPlayerPawn` 0))
  (bind _returnvalue_2 (`AIBlueprintHelperLibrary.GetBlackboard` (`AIBlueprintHelperLibrary.GetAIController` self)))
  ;[1 1 1] 距离与死亡更新
  (`parent.ReceiveTick` 0.0)
  (if (!= _returnvalue null)
    (`BlackboardComponent.SetValueAsBool` _returnvalue_2 (`self.CanAttack?_0`) (<= (`KismetMathLibrary.Vector_Distance2D` (`SceneComponent.K2_GetComponentLocation` (`self.Mesh`)) (`self.K2_GetActorLocation` _returnvalue)) 800.0))
    (`BlackboardComponent.SetValueAsBool` _returnvalue_2 (`self.IsDead?_0`) (`self.IsDead?`))
    (else
      (`BlackboardComponent.SetValueAsBool` _returnvalue_2 (`self.CanAttack?_0`) false))))

(event `self.AI Attack`
  ;[1 1 1] 攻击//c++以实现，蓝图作废
  (bind (_charactermovement _returnvalue) (`self.CanAttack?`))
  (if _returnvalue
    (set `self.IsAttacking` true)
    (`CharacterMovementComponent.SetMovementMode` _charactermovement "MOVE_None" 0)
    (`|PlayMontage` (`self.Mesh`) "/Game/Animations/Male_Anim_Axe_Combat_Swing_Montage.Male_Anim_Axe_Combat_Swing_Montage"
      (:`OnBlendOut`
        (if (== (`self.GetCurrentMontage`) null) :!label _label
          (`CharacterMovementComponent.SetMovementMode` _charactermovement "MOVE_Walking" 0)
          (set `self.IsAttacking` false)))
      (:`OnInterrupted`
        (goto _label))
      (:`OnNotifyBegin`
        ;[1 1 1] 法球球体碰撞
        (bind _returnvalue_2 (`|SpawnActorFromClass` "/Game/Character/BP_FireBallActor.BP_FireBallActor_C" (`SceneComponent.GetSocketTransform` (`self.Torch`) "Fire" "RTS_World") "AlwaysSpawn" "OverrideRootScale" null null))
        (`self.SetLifeSpan` _returnvalue_2 5.0)
        (bind _projectilemovement (`/Game/Character/BP_FireBallActor.ProjectileMovement` _returnvalue_2))
        (set `MovementComponent.Velocity` (* (`KismetMathLibrary.GetDirectionUnitVector` (`SceneComponent.K2_GetComponentLocation` (`self.Torch`)) (`self.K2_GetActorLocation` (`GameplayStatics.GetPlayerPawn` 0))) (`ProjectileMovementComponent.InitialSpeed` _projectilemovement)) _projectilemovement)
        (add `self.OnActorHit` _returnvalue_2 (delegate `OnActorHit_事件_0`))))))

(event `OnActorHit_事件_0` :!signature `self.OnActorHit`
  (params (SelfActor :type "Actor Object Reference") (OtherActor :type "Actor Object Reference") (NormalImpulse :type "Vector Structure") (Hit :type "HitResult Structure (by ref)"))
  ;[1 1 1] 法球球体碰撞
  (`self.K2_DestroyActor` SelfActor)
  ;[1 1 1] 播放受击动画
  (bind _asbp_blade_character (cast `/Game/Blueprints/BP_BladeCharacter` (`.HitActor` (`GameplayStatics.BreakHitResult` Hit))))
  (if (not (or (`self.ActorHasTag` _asbp_blade_character (`|GetArrayItem` (`self.Tags`))) (== (`self.GetCurrentMontage` _asbp_blade_character) "/Game/Animations/HIT_Montage.HIT_Montage")))
    (`self.TakeDamage` _asbp_blade_character (`self.Damage_0`))
    (bind _mesh (`Character.Mesh` _asbp_blade_character))
    (bind _returnvalue (- (`SceneComponent.K2_GetComponentLocation` (`self.Mesh`)) (`SceneComponent.K2_GetComponentLocation` _mesh)))
    (bind _returnvalue_2 (`KismetMathLibrary.Dot_VectorVector` _returnvalue (`SceneComponent.GetForwardVector` _mesh)))
    (if (>= _returnvalue_2 0.86)
      (bind _mesh_2 (`Character.Mesh` _asbp_blade_character))
      (`|PlayMontage` _mesh_2 "/Game/Animations/HIT_Montage.HIT_Montage" 1.0 0.0 "Back")
      (elif (<= _returnvalue_2 -0.86)
        (`|PlayMontage` _mesh_2 "/Game/Animations/HIT_Montage.HIT_Montage" 1.0 0.0 "Front")
        (elif (>= (`KismetMathLibrary.Dot_VectorVector` _returnvalue (`SceneComponent.GetRightVector` _mesh)) 0.0)
          (`|PlayMontage` _mesh_2 "/Game/Animations/HIT_Montage.HIT_Montage" 1.0 0.0 "Left")
          (else
            (`|PlayMontage` _mesh_2 "/Game/Animations/HIT_Montage.HIT_Montage" 1.0 0.0 "Right")))))))

(fn `UserConstructionScript`
  (`parent.UserConstructionScript`))